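; BP_Teleport is a teleporter that moves the player character from a Start volume to an Arrival point.
; On BeginPlay it caches the player pawn, cast to BP_ThirdPersonCharacter.
; When that character begins overlapping Start, it is instantly set to Arrival's world location with a non-swept teleport, and other actors are ignored.
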(event `self.ReceiveBeginPlay`
  (bind _asbp_third_person_character (cast `/Game/ThirdPerson/Blueprints/BP_ThirdPersonCharacter` (`GameplayStatics.GetPlayerPawn` 0)))
  (set `self.Player_Ref` _asbp_third_person_character))

(event `self.Start.OnComponentBeginOverlap`
  (params (OverlappedComponent :type "PrimitiveComponent Object Reference") (OtherActor :type "Actor Object Reference") (OtherComp :type "PrimitiveComponent Object Reference") (OtherBodyIndex :type Integer) (bFromSweep :type Boolean) (SweepResult :type "HitResult Structure (by ref)"))
  (if (== OtherActor (`self.Player_Ref`))
    (`self.K2_SetActorLocation` (`self.Player_Ref`) (`SceneComponent.K2_GetComponentLocation` (`self.Arrival`)) false true)))

(fn `UserConstructionScript`)