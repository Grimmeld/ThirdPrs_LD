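; BP_Interactable is a base interactable actor that offers itself to the player and shows a prompt widget when the player is near.
; Entering its Trigger registers it on the BP_ThirdPersonCharacter via SetUpInteractable and reveals the widget; leaving clears the registration and hides it.
; The widget turns toward the player's follow camera every tick.
; The Interact event is an empty hook with no behavior of its own.
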(event `self.ReceiveBeginPlay`
  (bind _asbp_third_person_character (cast `/Game/ThirdPerson/Blueprints/BP_ThirdPersonCharacter` (`GameplayStatics.GetPlayerPawn` 0)))
  (set `self.Player_Ref` _asbp_third_person_character)
  (`SceneComponent.SetHiddenInGame` (`self.Widget`) true false))

(event `Interact`)

(event `self.Trigger.OnComponentBeginOverlap`
  (params (OverlappedComponent :type "PrimitiveComponent Object Reference") (OtherActor :type "Actor Object Reference") (OtherComp :type "PrimitiveComponent Object Reference") (OtherBodyIndex :type Integer) (bFromSweep :type Boolean) (SweepResult :type "HitResult Structure (by ref)"))
  (if (== OtherActor (`self.Player_Ref`))
    (`/Game/ThirdPerson/Blueprints/BP_ThirdPersonCharacter.SetUpInteractable` (`self.Player_Ref`) self)
    (`SceneComponent.SetHiddenInGame` (`self.Widget`) false false)))

(event `self.Trigger.OnComponentEndOverlap`
  (params (OverlappedComponent :type "PrimitiveComponent Object Reference") (OtherActor :type "Actor Object Reference") (OtherComp :type "PrimitiveComponent Object Reference") (OtherBodyIndex :type Integer))
  (if (== OtherActor (`self.Player_Ref`))
    (`/Game/ThirdPerson/Blueprints/BP_ThirdPersonCharacter.SetUpInteractable` (`self.Player_Ref`) null)
    (`SceneComponent.SetHiddenInGame` (`self.Widget`) true false)))

(event `self.ReceiveTick`
  (params (DeltaSeconds :type "Float (single-precision)"))
  (bind _widget (`self.Widget`))
  (`SceneComponent.K2_SetWorldRotation` _widget (`KismetMathLibrary.FindLookAtRotation` (`SceneComponent.K2_GetComponentLocation` _widget) (`SceneComponent.K2_GetComponentLocation` (`/Game/ThirdPerson/Blueprints/BP_ThirdPersonCharacter.FollowCamera` (`self.Player_Ref`)))) false false))

(fn `UserConstructionScript`)