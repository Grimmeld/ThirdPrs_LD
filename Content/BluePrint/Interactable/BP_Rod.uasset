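; BP_Rod is an interactable rod pickup that the player collects.
; On Interact it calls GetRod on the player reference and AddObject on that player's HUD reference, then destroys itself.
; All logic lives in that single event, as BeginPlay, overlap and Tick are unused stubs and the construction script only calls its parent.
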(event `self.Interact`
  (bind _player_ref (`self.Player_Ref`))
  (`/Game/ThirdPerson/Blueprints/BP_ThirdPersonCharacter.GetRod` _player_ref)
  (`/Game/UI/WBP_HUD.AddObject` (`/Game/ThirdPerson/Blueprints/BP_ThirdPersonCharacter.HUD_ref` _player_ref))
  (`self.K2_DestroyActor`))

(fn `UserConstructionScript`
  (`parent.UserConstructionScript`))