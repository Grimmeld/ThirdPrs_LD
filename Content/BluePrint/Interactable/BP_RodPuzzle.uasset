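; BP_RodPuzzle is a one-time interactable puzzle that requires the player to have a rod.
; On Interact, a player with the rod is teleported to the Arrival component's location, the HUD object is cleared and the Rod component is revealed.
; Without the rod, the player gets a dialogue instead, and a Done flag blocks any interaction after success.
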(event `self.Interact`
  (bind _player_ref (`self.Player_Ref`))
  (if (`self.Done`)
    _
    (elif (`/Game/ThirdPerson/Blueprints/BP_ThirdPersonCharacter.hasRod` _player_ref)
      (`self.K2_SetActorLocation` _player_ref (`SceneComponent.K2_GetComponentLocation` (`self.Arrival`)) false true)
      (set `self.Done` true)
      (`/Game/UI/WBP_HUD.ClearObject` (`/Game/ThirdPerson/Blueprints/BP_ThirdPersonCharacter.HUD_ref` (`self.Player_Ref`)))
      (`SceneComponent.SetHiddenInGame` (`self.Rod`) false false)
      (else
        (`/Game/ThirdPerson/Blueprints/BP_ThirdPersonCharacter.CreateDialogue` _player_ref (`self.Dialogue`))))))

(fn `UserConstructionScript`
  (`parent.UserConstructionScript`))