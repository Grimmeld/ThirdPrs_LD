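; Interactable actor that teleports the player to a set arrival point, intended for moving across a wall.
; On Interact, it moves PlayerRef to the world location of its Arrival component with a teleport and no sweep.
; Each tick, after the parent's tick, it rotates its Widget to face the player's follow camera.
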(event `self.ReceiveTick`
  (params (DeltaSeconds :type "Float (single-precision)"))
  (bind _widget (`self.Widget`))
  (`parent.ReceiveTick` DeltaSeconds)
  (`SceneComponent.K2_SetWorldRotation` _widget (`KismetMathLibrary.FindLookAtRotation` (`SceneComponent.K2_GetComponentLocation` _widget) (`SceneComponent.K2_GetComponentLocation` (`/Game/ThirdPerson/Blueprints/BP_ThirdPersonCharacter.FollowCamera` (`self.Player_Ref`)))) false false))

(event `self.Interact`
  ; Move across the wall
  (`self.K2_SetActorLocation` (`self.Player_Ref`) (`SceneComponent.K2_GetComponentLocation` (`self.Arrival`)) false true))

(fn `UserConstructionScript`
  (`parent.UserConstructionScript`))