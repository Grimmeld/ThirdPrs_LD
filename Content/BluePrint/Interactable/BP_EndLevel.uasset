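; BP_EndLevel is an interactable actor that brings up the end-of-level screen when the player interacts with it.
; Its Interact event creates WBP_EndLevel for the local viewing controller of PlayerRef, adds it to the viewport and shows the mouse cursor on player controller 0.
; BeginPlay, overlap and Tick are disabled stubs, and the construction script only calls its parent.
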(event `self.Interact`
  (bind _returnvalue (`|CreateWidget` "/Game/UI/WBP_EndLevel.WBP_EndLevel_C" (`Pawn.GetLocalViewingPlayerController` (`self.Player_Ref`))))
  (`UserWidget.AddToViewport` _returnvalue 0)
  (set `PlayerController.bShowMouseCursor` true (`GameplayStatics.GetPlayerController` 0)))

(fn `UserConstructionScript`
  (`parent.UserConstructionScript`))