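; Interactable door actor that swings open once and has no closing logic.
; Interact plays the OpenDoor timeline to drive the Door's relative yaw, then sets IsOpened when it finishes, blocking further interaction.
; Tick rotates the Widget to face PlayerRef's follow camera and hides it once the door is open.
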(event `self.Interact`
  (if (not (`self.isOpened`))
    (bind (_direction _rotationdoor) (`Timeline|OpenDoor` :!via `PlayFromStart`)
      (:`Update`
        (`SceneComponent.K2_SetRelativeRotation` (`self.Door`) (`KismetMathLibrary.MakeRotator` 0.0 0.0 _rotationdoor) false false))
      (:`Finished`
        (set `self.isOpened` true)))))

(event `self.ReceiveTick`
  (params (DeltaSeconds :type "Float (single-precision)"))
  (bind _widget (`self.Widget`))
  (bind _widget_2 (`self.Widget`))
  ; If interacted, widget should be invisible
  (`|ExecutionSequence`
    (:`then_0`
      (if (`SceneComponent.bHiddenInGame` _widget)
        _
        (elif (`self.isOpened`)
          (`SceneComponent.SetHiddenInGame` _widget true false))))
    (:`then_1`
      (`SceneComponent.K2_SetWorldRotation` _widget_2 (`KismetMathLibrary.FindLookAtRotation` (`SceneComponent.K2_GetComponentLocation` _widget_2) (`SceneComponent.K2_GetComponentLocation` (`/Game/ThirdPerson/Blueprints/BP_ThirdPersonCharacter.FollowCamera` (`self.Player_Ref`)))) false false))))

(fn `UserConstructionScript`
  (`parent.UserConstructionScript`))